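; Actor Blueprint that computes and prints the factorial of Counter and opens a Fattoriale_WG widget when its Box is overlapped.
; The Fattoriale event loops from 1 to Counter minus 1, multiplying Number, seeded with Counter, by a DoN node's running count before printing the result on screen.
; The overlap creates a new widget each time; nothing in this graph calls Fattoriale.
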(event `Fattoriale`
  (set `self.Number` (`self.Counter`))
  (for _index (range 1 (`self.Counter`))
    (bind _counter (`/Engine/EditorBlueprintResources/StandardMacros.Do N` _index)
      (:`Exit`
        (set `self.Number` (* _counter (`self.Number`))))))
  (`KismetSystemLibrary.PrintString` (`KismetStringLibrary.Conv_IntToString` (`self.Number`)) true true (struct :`G` 0.66 :`B` 1.0 :`A` 1.0) 5.0))

(event `self.Box.OnComponentBeginOverlap`
  (params (OverlappedComponent :type "PrimitiveComponent Object Reference") (OtherActor :type "Actor Object Reference") (OtherComp :type "PrimitiveComponent Object Reference") (OtherBodyIndex :type Integer) (bFromSweep :type Boolean) (SweepResult :type "HitResult Structure (by ref)"))
  (bind _returnvalue (`|CreateWidget` "/Game/Fattoriale/Fattoriale_WG.Fattoriale_WG_C"))
  (`UserWidget.AddToViewport` _returnvalue 0))

(fn `UserConstructionScript`)