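; NumPrimo_BP is a Blueprint with a Box trigger that opens the NumPrimo_WG widget on overlap, apparently for a prime number check.
; The CalcoloNumPrimo event, not called within this Blueprint, runs nested modulo checks on Number against a few fixed divisors.
; It prints "Numero Primo" only when all of them divide Number, otherwise "Non un numero primo", so the test does not actually detect primes.
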(event `CalcoloNumPrimo`
  (if (== (mod (`self.Number`) 2) 0)
    (if (== (mod (`self.Number`) 3) 0)
      (if (== (mod (`self.Number`) 4) 0)
        (if (== (mod (`self.Number`) 5) 0)
          (if (== (mod (`self.Number`) 10) 0)
            (if (== (mod (`self.Number`) 11) 0)
              (`KismetSystemLibrary.PrintString` "Numero Primo")
              (else
                (`KismetSystemLibrary.PrintString` "Non un numero primo" :!label _label)))
            (else
              (goto _label)))
          (else
            (goto _label)))
        (else
          (goto _label)))
      (else
        (goto _label)))
    (else
      (goto _label))))

(event `self.Box.OnComponentBeginOverlap`
  (params (OverlappedComponent :type "PrimitiveComponent Object Reference") (OtherActor :type "Actor Object Reference") (OtherComp :type "PrimitiveComponent Object Reference") (OtherBodyIndex :type Integer) (bFromSweep :type Boolean) (SweepResult :type "HitResult Structure (by ref)"))
  (bind _returnvalue (`|CreateWidget` "/Game/NumeroPrimo/NumPrimo_WG.NumPrimo_WG_C"))
  (`UserWidget.AddToViewport` _returnvalue 0))

(fn `UserConstructionScript`)