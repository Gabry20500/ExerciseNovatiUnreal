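; Trigger actor that shows an Avarege_WG widget and provides an event for averaging an array of numbers.
; Any overlap with its Box creates a new widget in the viewport, and ending the overlap removes all widgets.
; The Mediadinnumeri event, not called within this graph, adds NumbArray into Sum without resetting it, divides by the array length and prints the result.
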(event `Media di n numeri`
  (bind _numbarray (`self.NumbArray`))
  (for _array_element _numbarray
    (set `self.Sum` (+ _array_element (`self.Sum`))))
  (bind _output_get (set `self.Avarage` (/ (`self.Sum`) (`KismetArrayLibrary.Array_Length` _numbarray))))
  (`KismetSystemLibrary.PrintString` (`KismetStringLibrary.Conv_IntToString` _output_get)))

(event `self.Box.OnComponentBeginOverlap`
  (params (OverlappedComponent :type "PrimitiveComponent Object Reference") (OtherActor :type "Actor Object Reference") (OtherComp :type "PrimitiveComponent Object Reference") (OtherBodyIndex :type Integer) (bFromSweep :type Boolean) (SweepResult :type "HitResult Structure (by ref)"))
  (bind _returnvalue (`|CreateWidget` "/Game/Avarage/Avarege_WG.Avarege_WG_C"))
  (`UserWidget.AddToViewport` _returnvalue 0))

(event `self.Box.OnComponentEndOverlap`
  (params (OverlappedComponent :type "PrimitiveComponent Object Reference") (OtherActor :type "Actor Object Reference") (OtherComp :type "PrimitiveComponent Object Reference") (OtherBodyIndex :type Integer))
  (`WidgetLayoutLibrary.RemoveAllWidgets`))

(fn `UserConstructionScript`)